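; BP_Comet is a comet actor that randomly picks one of two looks for its mesh.
; The construction script rolls a random integer, applies the first CometMaterial entry in most cases and the second otherwise, and records the choice in the Material boolean.
; BeginPlay is empty, so the asset has no runtime logic of its own.
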(event `self.ReceiveBeginPlay`)

(fn `UserConstructionScript`
  (if (< (`KismetMathLibrary.RandomIntegerInRange` 0 10) 8)
    (`PrimitiveComponent.SetMaterial` (`self.CometMesh`) 0 (`|GetArrayItem` (`self.CometMaterial`)))
    (set `self.bMaterial` false)
    (else
      (`PrimitiveComponent.SetMaterial` (`self.CometMesh`) 0 (`|GetArrayItem` (`self.CometMaterial`) 1))
      (set `self.bMaterial` true))))