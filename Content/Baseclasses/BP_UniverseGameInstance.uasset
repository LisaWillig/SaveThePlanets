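; Game instance that creates, loads and writes the game's SaveData save object for high score persistence.
; On Init it loads the save slot, or creates and saves a new object if none exists, setting HighScore to zero in both cases.
; SaveHighScore writes the held save object back to the slot without changing the score itself, printing the result for debugging.
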(event `self.ReceiveInit`
  (bind _returnvalue (`GameplayStatics.DoesSaveGameExist` (`self.SaveSlots`) (`self.UserID`)))
  (if _returnvalue
    (bind _returnvalue_2 (`GameplayStatics.LoadGameFromSlot` (`self.SaveSlots`) (`self.UserID`)))
    (bind _assave_data (cast `SaveData` _returnvalue_2))
    (set `self.SaveGameData` _assave_data)
    (set `self.HighScore` 0.0)
    (else
      (bind _returnvalue_3 (`GameplayStatics.CreateSaveGameObject` "/Script/SaveThePlanets.SaveData"))
      (bind _output_get (set `self.SaveGameData` _returnvalue_3))
      (set `self.HighScore` 0.0)
      (bind _returnvalue_4 (`GameplayStatics.SaveGameToSlot` _output_get (`self.SaveSlots`) (`self.UserID`)))
      (`KismetSystemLibrary.PrintString` (`KismetStringLibrary.Conv_BoolToString` _returnvalue_4)))))

(event `self.saveHighScore`
  (params (score :type "Float (single-precision)"))
  (bind _savegamedata (`self.SaveGameData`))
  (cast `SaveData` _savegamedata)
  (bind _returnvalue (`GameplayStatics.SaveGameToSlot` _savegamedata (`self.SaveSlots`) (`self.UserID`)))
  (`KismetSystemLibrary.PrintString` (`KismetStringLibrary.Conv_BoolToString` _returnvalue)))